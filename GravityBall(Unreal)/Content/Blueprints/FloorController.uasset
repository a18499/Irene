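; FloorController is a controller for a Floor pawn, with input meant to drive rotation.
; On BeginPlay it casts the controlled pawn to Floor and stores references to it and its Cube component.
; The MoveX axis, scaled by Initvalue and negated, forms an X-only vector converted through RotationFromXVector.
; That rotation is added locally to the controller actor itself; the stored Floor references go unused.
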(event EventBeginPlay
  (bind _asfloor (Utilities|Casting|CastToFloor (Pawn|GetControlledPawn)))
  (bind _output_get (Variables|Default|SetFlorinstance _asfloor))
  (Variables|Default|SetFloor (Variables|/Game/Floor.Floor_C|GetCube _output_get)))

(event Input|AxisEvents|InputAxisMoveX
  (params (AxisValue :type Float%20%28single-precision%29))
  (Transformation|AddActorLocalRotation (Math|Conversions|RotationFromXVector (Math|Vector|MakeVector (* AxisValue (Variables|Default|Getinitvalue) -1.0) 0.0 0.0)) false false))

(fn ConstructionScript)