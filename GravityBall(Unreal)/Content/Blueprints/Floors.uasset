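; Floor actor that the player tilts with movement input, enabled once something overlaps its trigger volume.
; MoveX and MoveY axes add scaled, inverted local roll and pitch to MainFloors, with no clamping.
; Pressing G sets the floor's relative rotation back to OrignPoint, and MoveX also prints the current rotation for debugging.
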(event OnComponentBeginOverlap(triggerVolume)
  (params (OtherActor :type Actor%20Object%20Reference) (OtherComp :type Primitive%20Component%20Object%20Reference) (OtherBodyIndex :type Integer) (bFromSweep :type Boolean) (SweepResult :type Hit%20Result%20Structure%20%28by%20ref%29))
  (Input|EnableInput (Game|GetPlayerController 0)))

(event Input|AxisEvents|InputAxisMoveX
  (params (AxisValue :type Float%20%28single-precision%29))
  (Transformation|AddLocalRotation (Variables|Default|GetMainFloors) (Math|Rotator|MakeRotator (* AxisValue (Variables|Default|Getinitvalue) -1.0) 0.0 0.0) false false)
  (Development|PrintString (Utilities|String|ToString(Rotator) (Variables|/Script/Engine.SceneComponent|GetRelativeRotation (Variables|Default|GetMainFloors))) (Variables|Default|GetTrue)))

(event Input|AxisEvents|InputAxisMoveY
  (params (AxisValue :type Float%20%28single-precision%29))
  (Transformation|AddLocalRotation (Variables|Default|GetMainFloors) (Math|Rotator|MakeRotator 0.0 (* AxisValue (Variables|Default|Getinitvalue) -1.0) 0.0) false false))

(event Input|KeyboardEvents|G
  (params (Key :type Key%20Structure :default "AnyKey"))
  (:Pressed
    (Transformation|SetRelativeRotation (Variables|Default|GetMainFloors) (Variables|Default|GetOrignPoint) false false)))

(fn ConstructionScript)